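; A level exit trigger volume that advances the game once every crystal in the level is collected.
; On overlap by an actor passing the IsActor check, it counts remaining BP_Crystal actors and prints a reminder if any are left.
; Otherwise it finds the current level's name in LevelList and opens the following entry, or quits the game on the last one.
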(event OnComponentBeginOverlap(Collision)
  (params (OverlappedComponent :type Primitive%20Component%20Object%20Reference) (OtherActor :type Actor%20Object%20Reference) (OtherComp :type Primitive%20Component%20Object%20Reference) (OtherBodyIndex :type Integer) (bFromSweep :type Boolean) (SweepResult :type Hit%20Result%20Structure%20%28by%20ref%29))
  (Utilities|IsValid OtherActor
    (:Is%20Valid
      (Utilities|IsActor OtherActor
        (:True
          (if (CallFunction|CheckAnyCrystals)
            (Utilities|IsLastIndex
              (:Return
                (CallFunction|NextLevel)))
            (else
              (Development|PrintString "Get all the crystals!" true true "(R=0.229615,G=0.000000,B=0.287500,A=1.000000)"))))))))

(fn ConstructionScript)

(fn CheckAnyCrystals
  (bind _outactors (Actor|GetAllActorsOfClass "/Game/Blueprints/Actors/Collectables/BP_Crystal.BP_Crystal_C"))
  (return (== (Utilities|Array|Length _outactors) 0)))

(fn CheckIndex
  (bind _returnvalue (Game|GetCurrentLevelName true))
  (return (Utilities|Array|FindItem (Variables|Default|GetLevelList) (Utilities|String|StringToName _returnvalue))))

(fn NextLevel
  (Game|OpenLevel(byName) (Utilities|Array|Get(acopy) (Variables|Default|GetLevelList) (+ (CallFunction|CheckIndex) 1))))