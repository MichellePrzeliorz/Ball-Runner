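; BP_Crystal is a collectable crystal that flies into the player and vanishes when the player touches its sphere.
; On overlap it caches its location, scale and light intensity, then plays the CrystalTimeMovement timeline.
; The timeline's tracks lerp the crystal toward the pawn's live location while shrinking it and fading its point light, then it destroys itself.
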(event OnComponentBeginOverlap(Sphere)
  (params (OverlappedComponent :type Primitive%20Component%20Object%20Reference) (OtherActor :type Actor%20Object%20Reference) (OtherComp :type Primitive%20Component%20Object%20Reference) (OtherBodyIndex :type Integer) (bFromSweep :type Boolean) (SweepResult :type Hit%20Result%20Structure%20%28by%20ref%29))
  (Utilities|IsActor OtherActor
    (:True
      (CallFunction|SetProperties)
      (bind (_direction _lerpmovement _lerpscale _lerplight) (Timeline|CrystalTimeMovement Play)
        (:Update
          (CallFunction|LokalizacjaKryształu _lerpmovement)
          (CallFunction|SkalaKryształu _lerpscale)
          (CallFunction|MruganieKryształu _lerplight))
        (:Finished
          (Actor|DestroyActor))))))

(fn ConstructionScript)

(fn PrzesuwanieKryształuWStronęGracza
  (params (Alpha :type Float%20%28single-precision%29) (Alpha2 :type Float%20%28single-precision%29))
  (Transformation|SetActorLocation (Math|Vector|Lerp(Vector) (Transformation|GetActorLocation) (Transformation|GetActorLocation (Game|Player|GetPlayerPawn 0)) Alpha) false false)
  (Transformation|SetActorScale3D (Math|Vector|Lerp(Vector) (Transformation|GetActorScale3D) "0, 0, 0" Alpha2))
  (CallFunction|NewFunction0))

(fn MruganieKryształu
  (params (Alpha :type Float%20%28single-precision%29))
  (Rendering|Components|Light|SetIntensity (Variables|Default|GetPointLight) (Math|Float|Lerp (Variables|CrystalProperties|GetCrystalIntensity) 0.0 Alpha)))

(fn NewFunction0
  (bind _pointlight (Variables|Default|GetPointLight))
  (Rendering|Components|Light|SetIntensity _pointlight (Math|Float|Lerp (Variables|/Script/Engine.LightComponentBase|GetIntensity _pointlight) 0.0 0.0)))

(fn SkalaKryształu
  (params (Alpha :type Float%20%28single-precision%29))
  (Transformation|SetActorScale3D (Math|Vector|Lerp(Vector) (Variables|CrystalProperties|GetCrystalScale) "0, 0, 0" Alpha)))

(fn LokalizacjaKryształu
  (params (Alpha :type Float%20%28single-precision%29))
  (Transformation|SetActorLocation (Math|Vector|Lerp(Vector) (Variables|CrystalProperties|GetCrystalLocation) (Transformation|GetActorLocation (Game|Player|GetPlayerPawn 0)) Alpha) false false))

(fn SetProperties
  (Variables|CrystalProperties|SetCrystalLocation (Transformation|GetActorLocation))
  (Variables|CrystalProperties|SetCrystalScale (Transformation|GetActorScale3D))
  (Variables|CrystalProperties|SetCrystalIntensity (Variables|/Script/Engine.LightComponentBase|GetIntensity (Variables|Default|GetPointLight))))